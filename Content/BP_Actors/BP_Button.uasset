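; Interactable button actor that shows an "E to interact" prompt and announces presses through an event dispatcher.
; Interacting prints a debug string and runs TurnOnAndOff, which calls the pressed dispatcher and plays a timeline that slides the Button along X by the negated TurnKnob value.
; The construction script rolls the Button by the On flag, which interaction never changes.
; The pickup rotation and scale functions return zero vectors.
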(event `TurnOnAndOff`
  (`self.PressedDispatcher`)
  (bind (_direction _turnknob) (`Timeline|On/Off Timeline` :`NewTime` 0.1)
    (:`Update`
      (`SceneComponent.K2_SetRelativeLocation` (`self.button`) (`KismetMathLibrary.MakeVector` (* _turnknob -1.0)) false false))))

(fn `InteractWith`
  (params (Interactor :type "/Game/Blueprints/BP_FirstPersonCharacter Object Reference") (HitComponent :type "PrimitiveComponent Object Reference"))
  (returns (CanGrab :type Boolean))
  (`KismetSystemLibrary.PrintString` "Hs Interacted")
  (`self.TurnOnAndOff`)
  (return false))

(fn `LookAt`
  (params (Interactor :type "/Game/Blueprints/BP_FirstPersonCharacter Object Reference") (HitComponent :type "PrimitiveComponent Object Reference") (Controller :type "PlayerController Object Reference"))
  (returns (LookAtActor :type "Actor Object Reference") (LookAtComponent :type "PrimitiveComponent Object Reference") (Message :type Text) (CanInteract :type Boolean))
  (return self HitComponent "E to interact" true))

(fn `PickupRotation`
  (returns (PickupRotation :type "Rotator Structure"))
  (return))

(fn `PickupScale`
  (returns (Scale :type "Vector Structure"))
  (return (0.0 0.0 0.0)))

(fn `UserConstructionScript`
  (bind _button (`self.button`))
  (if (`self.On`)
    (`SceneComponent.K2_SetRelativeRotation` _button (`KismetMathLibrary.MakeRotator` -90.0) false false)
    (else
      (`SceneComponent.K2_SetRelativeRotation` _button (`KismetMathLibrary.MakeRotator` 0.0) false false))))
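; BP_Carrot_Bottom is a sliceable carrot-bottom food actor that breaks into smaller pieces when cut.
; When its FoodItem component begins overlapping a component tagged "Slice", it calls the Split event.
; Split spawns two BP_Carrot_Piece actors, both at FoodItem's world transform, then destroys the original actor.
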(event `Split`
  (bind _returnvalue (`SceneComponent.K2_GetComponentToWorld` (`self.FoodItem`)))
  (`|SpawnActorFromClass` "/Game/BP_Actors/BP_Carrot_Piece.BP_Carrot_Piece_C" _returnvalue "Undefined" "OverrideRootScale" null null)
  (`|SpawnActorFromClass` "/Game/BP_Actors/BP_Carrot_Piece.BP_Carrot_Piece_C" _returnvalue "Undefined" "OverrideRootScale" null null)
  (`self.K2_DestroyActor`))

(event `self.FoodItem.OnComponentBeginOverlap`
  (params (OverlappedComponent :type "PrimitiveComponent Object Reference") (OtherActor :type "Actor Object Reference") (OtherComp :type "PrimitiveComponent Object Reference") (OtherBodyIndex :type Integer) (bFromSweep :type Boolean) (SweepResult :type "HitResult Structure (by ref)"))
  (if (`ActorComponent.ComponentHasTag` OtherComp "Slice")
    (`self.Split`)))

(fn `UserConstructionScript`
  (`parent.UserConstructionScript`))
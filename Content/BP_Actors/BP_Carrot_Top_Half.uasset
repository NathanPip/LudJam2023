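; BP_Carrot_Top_Half is a choppable food actor for the top half of a carrot, applying its material to the FoodItem component on BeginPlay.
; An overlap with a component tagged "Slice" calls Split, which plays a chop sound and spawns two carrot pieces and a carrot top at the food's transform.
; Each spawned actor inherits the CookAmt and refreshes its cook material before the original destroys itself.
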(event `self.ReceiveBeginPlay`
  (`parent.ReceiveBeginPlay`)
  (`PrimitiveComponent.SetMaterial` (`self.FoodItem`) 0 (`self.MaterialInstance`)))

(event `Split`
  (bind _returnvalue (`SceneComponent.K2_GetComponentToWorld` (`self.FoodItem`)))
  (`GameplayStatics.PlaySoundAtLocation` "/Game/Sounds/SFX_Chop_Cue.SFX_Chop_Cue" (`self.K2_GetActorLocation`) (struct) 1.0 1.0 0.0 null null null null)
  (bind _returnvalue_2 (`|SpawnActorFromClass` "/Game/BP_Actors/BP_Carrot_Piece.BP_Carrot_Piece_C" _returnvalue "Undefined" "OverrideRootScale" null null))
  (set `/Game/BP_Actors/BPB_Food_Item.cookAmt` (`self.cookAmt`) _returnvalue_2)
  (`self.SetCookMaterial` _returnvalue_2)
  (bind _returnvalue_3 (`|SpawnActorFromClass` "/Game/BP_Actors/BP_Carrot_Piece.BP_Carrot_Piece_C" _returnvalue "Undefined" "OverrideRootScale" null null))
  (set `/Game/BP_Actors/BPB_Food_Item.cookAmt` (`self.cookAmt`) _returnvalue_3)
  (`self.SetCookMaterial` _returnvalue_3)
  (bind _returnvalue_4 (`|SpawnActorFromClass` "/Game/BP_Actors/BP_Carrot_Top.BP_Carrot_Top_C" _returnvalue "Undefined" "OverrideRootScale" null null))
  (set `/Game/BP_Actors/BPB_Food_Item.cookAmt` (`self.cookAmt`) _returnvalue_4)
  (`self.SetCookMaterial` _returnvalue_4)
  (`self.K2_DestroyActor`))

(event `self.FoodItem.OnComponentBeginOverlap`
  (params (OverlappedComponent :type "PrimitiveComponent Object Reference") (OtherActor :type "Actor Object Reference") (OtherComp :type "PrimitiveComponent Object Reference") (OtherBodyIndex :type Integer) (bFromSweep :type Boolean) (SweepResult :type "HitResult Structure (by ref)"))
  (if (`ActorComponent.ComponentHasTag` OtherComp "Slice")
    (`self.Split`)))

(fn `UserConstructionScript`
  (`parent.UserConstructionScript`))
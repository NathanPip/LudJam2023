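; Cat actor Coots, which moves to its feeding spot to eat, then turns to watch the player.
; BeginPlay caches the anim Blueprint, the CootsFeedingSpot transform and the game mode's CootsMeals.
; MoveToFood sets IsEating and lerps the cat to the spot by timeline, then CheckFood rolls the mesh.
; When the roll finishes, RotateToPlayer makes Tick aim the mesh at the player.
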(event `self.ReceiveBeginPlay`
  (bind _ascat_anim_blueprint (cast `/Game/Models/cat/CatAnimBlueprint` (`SkeletalMeshComponent.GetAnimInstance` (`self.Coots`))))
  (set `self.Animation Blueprint` _ascat_anim_blueprint)
  (bind _returnvalue (`GameplayStatics.GetActorOfClass` "/Game/BP_Actors/CootsFeedingSpot.CootsFeedingSpot_C"))
  (bind _defaultsceneroot (`/Game/BP_Actors/CootsFeedingSpot.DefaultSceneRoot` _returnvalue))
  (set `self.Coots Eating Spot` (`KismetMathLibrary.MakeTransform` (`SceneComponent.K2_GetComponentLocation` _defaultsceneroot) (`SceneComponent.K2_GetComponentRotation` _defaultsceneroot)))
  (bind _asbp_first_person_game_mode (cast `/Game/FirstPerson/Blueprints/BP_FirstPersonGameMode` (`GameplayStatics.GetGameMode`)))
  (set `self.Coots Meals` (`/Game/FirstPerson/Blueprints/BP_FirstPersonGameMode.CootsMeals` _asbp_first_person_game_mode)))

(event `self.ReceiveTick`
  (params (DeltaSeconds :type "Float (single-precision)"))
  (bind (_returnvalue_roll _returnvalue_pitch _returnvalue_yaw) (`KismetMathLibrary.BreakRotator` (`KismetMathLibrary.FindLookAtRotation` (`SceneComponent.K2_GetComponentLocation` (`self.Coots`)) (`self.K2_GetActorLocation` (`GameplayStatics.GetPlayerPawn` 0)))))
  (if (`self.RotateToPlayer`)
    (`SceneComponent.K2_SetRelativeRotation` (`self.Coots`) (`KismetMathLibrary.MakeRotator` _returnvalue_roll _returnvalue_pitch _returnvalue_yaw) false false)))

(event `MoveToFood`
  (bind _coots (`self.Coots`))
  (bind _coots_eating_spot (`self.Coots Eating Spot`))
  (bind _relativelocation_x (`KismetMathLibrary.BreakVector` (`SceneComponent.RelativeLocation` _coots)))
  (set `/Game/Models/cat/CatAnimBlueprint.isEating` true (`self.Animation Blueprint`))
  (bind (_direction _newtrack_0) (`Timeline|To Food` :!via `PlayFromStart`)
    (:`Update`
      (`self.K2_SetActorLocation` (`KismetMathLibrary.VLerp` (`self.K2_GetActorLocation`) (`KismetMathLibrary.MakeVector` (.x (.location _coots_eating_spot)) (.y (.location _coots_eating_spot)) (+ (.z (.location _coots_eating_spot)) 3.0)) _newtrack_0))
      (`self.K2_SetActorRotation` (`KismetMathLibrary.RLerp` (`self.K2_GetActorRotation`) (.rotation _coots_eating_spot) _newtrack_0))
      (`SceneComponent.K2_SetRelativeLocation` _coots (`KismetMathLibrary.MakeVector` (`KismetMathLibrary.Lerp` _relativelocation_x -80.0 _newtrack_0)) false false))
    (:`Finished`
      (`self.CheckFood`))))

(event `CheckFood`
  (bind _coots (`self.Coots`))
  (bind (_relativerotation_roll _relativerotation_pitch _relativerotation_yaw) (`KismetMathLibrary.BreakRotator` (`SceneComponent.RelativeRotation` _coots)))
  (bind (_direction _newtrack_0) (`Timeline|RotateTimeLine` :!via `PlayFromStart`)
    (:`Update`
      (`SceneComponent.K2_SetRelativeRotation` _coots (`KismetMathLibrary.MakeRotator` (`KismetMathLibrary.Lerp` 0.0 60.0 _newtrack_0) _relativerotation_pitch _relativerotation_yaw) false false))
    (:`Finished`
      (set `self.RotateToPlayer` true)
      (`Timeline|LookAtTimeline` :!via `PlayFromStart`))))

(fn `UserConstructionScript`)
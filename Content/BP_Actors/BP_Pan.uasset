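; Pan actor that can be picked up, heats up from a heat source and passes that heat to overlapping actors.
; EnterHeat and ExitHeat toggle heating and cooling, which Tick integrates into HeatAmt up to a source-scaled limit.
; HeatAmt drives the emissive glow on a dynamic material created in the Construction Script.
; While hot, Tick sends heat messages to BPI_Interaction actors inside Heat_collision, otherwise exit messages.
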(event `self.ReceiveTick`
  (params (DeltaSeconds :type "Float (single-precision)"))
  (`|ExecutionSequence`
    (:`then_0`
      (if (`self.isHeating`)
        (bind _output_get (set `self.HeatAmt` (+ (* (* (`self.HeatingAmount`) (`self.HeatScalar`)) DeltaSeconds) (`self.HeatAmt`))))
        (if (< _output_get (* (`self.HeatScalar`) (`self.MaxHeatMultiplier`)))
          (set `self.isHot` true)
          (`MaterialInstanceDynamic.SetScalarParameterValue` (`self.MaterialInstance`) "EmissiveStrength" (* (`self.HeatAmt`) 0.001) :!label _label)
          (else
            (set `self.isHeating` false)))))
    (:`then_1`
      (if (`self.isCooling`)
        (bind _output_get_2 (set `self.HeatAmt` (- (`self.HeatAmt`) (* (`self.CoolingAmount`) DeltaSeconds))))
        (if (> _output_get_2 5.0)
          (goto _label)
          (else
            (set `self.isCooling` false)
            (set `self.HeatAmt` 0.0)
            (set `self.isHot` false)
            (goto _label)))))
    (:`then_2`
      (if (> (`KismetArrayLibrary.Array_Length` (`self.overlappedActors`)) 0)
        (if (`self.isHot`)
          (for _array_element (`self.overlappedActors`)
            (message `/Game/Interfaces/BPI_Interaction.EnterHeat` _array_element (`self.HeatAmt`)))
          (elif true
            (for _array_element_2 (`self.overlappedActors`)
              (message `/Game/Interfaces/BPI_Interaction.ExitHeat` _array_element_2))))))))

(event `/Game/Interfaces/BPI_Interaction.EnterHeat`
  (params (Heat :type "Float (double-precision)"))
  (bind _output_get (set `self.HeatScalar` Heat))
  (set `self.isCooling` false)
  (set `self.isHeating` true)
  (`KismetSystemLibrary.PrintString` (`KismetStringLibrary.Conv_DoubleToString` _output_get)))

(event `/Game/Interfaces/BPI_Interaction.ExitHeat`
  (set `self.HeatScalar` 0.0)
  (set `self.isHeating` false)
  (set `self.isCooling` true)
  (`KismetSystemLibrary.PrintString` "cooling"))

(event `self.heat_collision.OnComponentBeginOverlap`
  (params (OverlappedComponent :type "PrimitiveComponent Object Reference") (OtherActor :type "Actor Object Reference") (OtherComp :type "PrimitiveComponent Object Reference") (OtherBodyIndex :type Integer) (bFromSweep :type Boolean) (SweepResult :type "HitResult Structure (by ref)"))
  (if (`KismetSystemLibrary.DoesImplementInterface` OtherActor "/Game/Interfaces/BPI_Interaction.BPI_Interaction_C")
    (`KismetArrayLibrary.Array_Add` (`self.overlappedActors`) OtherActor)))

(event `self.heat_collision.OnComponentEndOverlap`
  (params (OverlappedComponent :type "PrimitiveComponent Object Reference") (OtherActor :type "Actor Object Reference") (OtherComp :type "PrimitiveComponent Object Reference") (OtherBodyIndex :type Integer))
  (bind _overlappedactors (`self.overlappedActors`))
  (if (`KismetArrayLibrary.Array_Contains` _overlappedactors OtherActor)
    (message `/Game/Interfaces/BPI_Interaction.ExitHeat` OtherActor)
    (`KismetArrayLibrary.Array_RemoveItem` _overlappedactors OtherActor)))

(fn `InteractWith`
  (params (Interactor :type "/Game/Blueprints/BP_FirstPersonCharacter Object Reference") (HitComponent :type "PrimitiveComponent Object Reference"))
  (returns (CanGrab :type Boolean))
  (return true))

(fn `LookAt`
  (params (Interactor :type "/Game/Blueprints/BP_FirstPersonCharacter Object Reference") (HitComponent :type "PrimitiveComponent Object Reference") (Controller :type "PlayerController Object Reference"))
  (returns (LookAtActor :type "Actor Object Reference") (LookAtComponent :type "PrimitiveComponent Object Reference") (Message :type Text) (CanInteract :type Boolean))
  (return self HitComponent "E to Pick Up" true))

(fn `PickupRotation`
  (returns (PickupRotation :type "Rotator Structure"))
  (return (struct :`Yaw` 90.0)))

(fn `PickupScale`
  (returns (Scale :type "Vector Structure"))
  (return (0.5 0.5 0.5)))

(fn `UserConstructionScript`
  (bind _returnvalue (`PrimitiveComponent.CreateDynamicMaterialInstance` (`self.pan_mesh`) 0 "/Game/Models/Pan/mat_pan.mat_pan" "None"))
  (set `self.MaterialInstance` _returnvalue))
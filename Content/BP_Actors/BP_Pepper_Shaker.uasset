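; Pepper shaker actor that can be picked up and tilted to pepper food items.
; On Tick, a mesh roll beyond 25 degrees either way activates the pepper emitter and box-traces from it to an end-point component.
; A hit BPB_Food_Item receives Pepper every frame, and the emitter deactivates when upright.
; Interaction functions supply the pickup prompt, rotation and half scale.
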(event `self.ReceiveTick`
  (params (DeltaSeconds :type "Float (single-precision)"))
  (bind _pepperemitter (`self.PepperEmitter`))
  (bind _relativerotation_roll (`KismetMathLibrary.BreakRotator` (`SceneComponent.RelativeRotation` (`self.salt_shaker_mesh`))))
  (if (> (`KismetMathLibrary.Abs` _relativerotation_roll) 25.0)
    (bind _outhit (`KismetSystemLibrary.BoxTraceSingle` (`SceneComponent.K2_GetComponentLocation` (`self.PepperEmitter`)) (`SceneComponent.K2_GetComponentLocation` (`self.EmissionEndPoint`)) (2.0 2.0 2.0) (struct) "TraceTypeQuery1"))
    (`ActorComponent.Activate` _pepperemitter false)
    (bind _asbpb_food_item (cast `/Game/BP_Actors/BPB_Food_Item` (`.HitActor` (`GameplayStatics.BreakHitResult` _outhit))))
    (`/Game/BP_Actors/BPB_Food_Item.Pepper` _asbpb_food_item)
    (else
      (`ActorComponent.Deactivate` _pepperemitter))))

(fn `InteractWith`
  (params (Interactor :type "/Game/Blueprints/BP_FirstPersonCharacter Object Reference") (HitComponent :type "PrimitiveComponent Object Reference"))
  (returns (CanGrab :type Boolean))
  (return true))

(fn `LookAt`
  (params (Interactor :type "/Game/Blueprints/BP_FirstPersonCharacter Object Reference") (HitComponent :type "PrimitiveComponent Object Reference") (Controller :type "PlayerController Object Reference"))
  (returns (LookAtActor :type "Actor Object Reference") (LookAtComponent :type "PrimitiveComponent Object Reference") (Message :type Text) (CanInteract :type Boolean))
  (return self HitComponent "Press E To Pick Up" true))

(fn `PickupRotation`
  (returns (PickupRotation :type "Rotator Structure"))
  (return))

(fn `PickupScale`
  (returns (Scale :type "Vector Structure"))
  (return (0.5 0.5 0.5)))

(fn `UserConstructionScript`)
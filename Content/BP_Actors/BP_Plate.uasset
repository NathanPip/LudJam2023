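; BP_Plate is a plate actor that, when flagged as a feeding plate, receives cat food and summons BP_Coots to it.
; When a BP_CatFood overlaps FoodCollision, it stores the food on itself and the first-person game mode, drops it, then calls MoveToFood on Coots.
; Interaction, pickup and food-value functions return empty defaults, and the FoodPlaced, EatFood and TossFood events are empty.
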(event `self.ReceiveBeginPlay`)

(event `FoodPlaced`
  (params (CatFood :type "/Game/BP_Actors/BP_CatFood Object Reference")))

(event `self.FoodCollision.OnComponentBeginOverlap`
  (params (OverlappedComponent :type "PrimitiveComponent Object Reference") (OtherActor :type "Actor Object Reference") (OtherComp :type "PrimitiveComponent Object Reference") (OtherBodyIndex :type Integer) (bFromSweep :type Boolean) (SweepResult :type "HitResult Structure (by ref)"))
  (if (`self.IsFeedingPlate`)
    (bind _asbp_cat_food (cast `/Game/BP_Actors/BP_CatFood` OtherActor))
    (set `self.CatFood` _asbp_cat_food)
    (bind _asbp_first_person_game_mode (cast `/Game/FirstPerson/Blueprints/BP_FirstPersonGameMode` (`GameplayStatics.GetGameMode`)))
    (set `/Game/FirstPerson/Blueprints/BP_FirstPersonGameMode.CatFood` _asbp_cat_food _asbp_first_person_game_mode)
    (`/Game/Interfaces/BPI_Interaction.Drop` _asbp_cat_food)
    (bind _returnvalue (`GameplayStatics.GetActorOfClass` "/Game/BP_Actors/BP_Coots.BP_Coots_C"))
    (`/Game/BP_Actors/BP_Coots.MoveToFood` _returnvalue)))

(event `EatFood`)

(event `TossFood`)

(fn `getFoodValues`
  (returns (cookAmt :type "Float (double-precision)") (pepperAmt :type "Float (double-precision)") (saltAmt :type "Float (double-precision)"))
  (return 0.0 0.0 0.0))

(fn `InteractWith`
  (params (Interactor :type "/Game/Blueprints/BP_FirstPersonCharacter Object Reference") (HitComponent :type "PrimitiveComponent Object Reference"))
  (returns (CanGrab :type Boolean))
  (return false))

(fn `LookAt`
  (params (Interactor :type "/Game/Blueprints/BP_FirstPersonCharacter Object Reference") (HitComponent :type "PrimitiveComponent Object Reference") (Controller :type "PlayerController Object Reference"))
  (returns (LookAtActor :type "Actor Object Reference") (LookAtComponent :type "PrimitiveComponent Object Reference") (Message :type Text) (CanInteract :type Boolean))
  (return self HitComponent "" false))

(fn `PickupRotation`
  (returns (PickupRotation :type "Rotator Structure"))
  (return))

(fn `PickupScale`
  (returns (Scale :type "Vector Structure"))
  (return (0.0 0.0 0.0)))

(fn `UserConstructionScript`)
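; BP_blueberry is a blueberry food item actor that presents itself as something the player can pick up.
; On BeginPlay it applies a material instance to its FoodItem component.
; Interaction functions show an "E To Pick Up" prompt on look-at and return true on interact, with no pickup logic in this graph.
; PickupRotation and PickupScale supply a zero rotation and a half-size scale for the picked-up item.
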(event `self.ReceiveBeginPlay`
  (`PrimitiveComponent.SetMaterial` (`self.FoodItem`) 0 (`self.MaterialInstance`)))

(fn `InteractWith`
  (params (Interactor :type "/Game/Blueprints/BP_FirstPersonCharacter Object Reference") (HitComponent :type "PrimitiveComponent Object Reference"))
  (returns (CanGrab :type Boolean))
  (return true))

(fn `LookAt`
  (params (Interactor :type "/Game/Blueprints/BP_FirstPersonCharacter Object Reference") (HitComponent :type "PrimitiveComponent Object Reference") (Controller :type "PlayerController Object Reference"))
  (returns (LookAtActor :type "Actor Object Reference") (LookAtComponent :type "PrimitiveComponent Object Reference") (Message :type Text) (CanInteract :type Boolean))
  (return self HitComponent "E To Pick Up" true))

(fn `PickupRotation`
  (returns (PickupRotation :type "Rotator Structure"))
  (return))

(fn `PickupScale`
  (returns (Scale :type "Vector Structure"))
  (return (0.5 0.5 0.5)))

(fn `UserConstructionScript`)
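; Interactable faucet knob that toggles on and off when used, with a fixed "E To Turn On" look-at prompt.
; InteractWith calls the toggle, which flips the On state and fires an on/off dispatcher for listeners.
; A timeline plays or reverses to lerp the knob's yaw by a scaled rotation amount, printing its alpha on each update.
; Pickup rotation and scale functions return zero vectors.
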(event `Turn On/Off`
  (bind _knob_one (`self.KNOB_ONE`))
  (bind (_relativerotation_roll _relativerotation_pitch) (`KismetMathLibrary.BreakRotator` (`SceneComponent.RelativeRotation` _knob_one)))
  (bind _output_get (set `self.On` (!= (`self.On`) true)))
  (`self.OnOffDispatcher`)
  (if _output_get
    (bind (_direction _rotate) (`Timeline|RotateTimeline` :!label _label)
      (:`Update`
        (`SceneComponent.K2_SetRelativeRotation` _knob_one (`KismetMathLibrary.MakeRotator` _relativerotation_roll _relativerotation_pitch (`KismetMathLibrary.Lerp` 0.0 (* (`self.RotAmt`) (`self.RotMultiplier`)) _rotate)) false false)
        (`KismetSystemLibrary.PrintString` (`KismetStringLibrary.Conv_DoubleToString` _rotate))))
    (else
      (goto _label :!via `Reverse`))))

(fn `InteractWith`
  (params (Interactor :type "/Game/Blueprints/BP_FirstPersonCharacter Object Reference") (HitComponent :type "PrimitiveComponent Object Reference"))
  (returns (CanGrab :type Boolean))
  (`self.Turn On/Off`)
  (return false))

(fn `LookAt`
  (params (Interactor :type "/Game/Blueprints/BP_FirstPersonCharacter Object Reference") (HitComponent :type "PrimitiveComponent Object Reference") (Controller :type "PlayerController Object Reference"))
  (returns (LookAtActor :type "Actor Object Reference") (LookAtComponent :type "PrimitiveComponent Object Reference") (Message :type Text) (CanInteract :type Boolean))
  (return self HitComponent "E To Turn On" true))

(fn `PickupRotation`
  (returns (PickupRotation :type "Rotator Structure"))
  (return))

(fn `PickupScale`
  (returns (Scale :type "Vector Structure"))
  (return (0.0 0.0 0.0)))

(fn `UserConstructionScript`)
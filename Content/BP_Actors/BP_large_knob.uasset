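; Interactable large stove knob that toggles between on and off, with an "E to interact" prompt when looked at.
; Interacting prints a debug string, flips the On state, calls an on/off dispatcher, and plays or reverses a timeline that lerps the knob's roll toward RotationAmount.
; The construction script poses the knob from On using a hardcoded roll rather than RotationAmount.
; Pickup rotation and scale functions return zero vectors.
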(event `TurnOnAndOff`
  (bind _output_get (set `self.On` (!= (`self.On`) true)))
  (`self.OnOffDispatcher`)
  (if _output_get
    (bind (_direction _turnknob) (`Timeline|On/Off Timeline` :`NewTime` 0.1 :!label _label)
      (:`Update`
        (`SceneComponent.K2_SetRelativeRotation` (`self.stove_large_knob`) (`KismetMathLibrary.MakeRotator` (`KismetMathLibrary.Lerp` 0.0 (`self.RotationAmount`) _turnknob)) false false)))
    (else
      (goto _label :!via `Reverse`))))

(fn `InteractWith`
  (params (Interactor :type "/Game/Blueprints/BP_FirstPersonCharacter Object Reference") (HitComponent :type "PrimitiveComponent Object Reference"))
  (returns (CanGrab :type Boolean))
  (`KismetSystemLibrary.PrintString` "Hs Interacted")
  (`self.TurnOnAndOff`)
  (return false))

(fn `LookAt`
  (params (Interactor :type "/Game/Blueprints/BP_FirstPersonCharacter Object Reference") (HitComponent :type "PrimitiveComponent Object Reference") (Controller :type "PlayerController Object Reference"))
  (returns (LookAtActor :type "Actor Object Reference") (LookAtComponent :type "PrimitiveComponent Object Reference") (Message :type Text) (CanInteract :type Boolean))
  (return self HitComponent "E to interact" true))

(fn `PickupRotation`
  (returns (PickupRotation :type "Rotator Structure"))
  (return))

(fn `PickupScale`
  (returns (Scale :type "Vector Structure"))
  (return (0.0 0.0 0.0)))

(fn `UserConstructionScript`
  (bind _stove_large_knob (`self.stove_large_knob`))
  (if (`self.On`)
    (`SceneComponent.K2_SetRelativeRotation` _stove_large_knob (`KismetMathLibrary.MakeRotator` -90.0) false false)
    (else
      (`SceneComponent.K2_SetRelativeRotation` _stove_large_knob (`KismetMathLibrary.MakeRotator` 0.0) false false))))
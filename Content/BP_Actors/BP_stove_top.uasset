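; Stove top actor that toggles on and off, acting as a heat source for other objects in the game.
; Toggling sends enter or exit heat messages through BPI_Interaction to actors overlapping its heat collider, and overlap events update actors that arrive or leave.
; A timeline plays or reverses on toggle, driving emissive strength on a dynamic material instance created in the construction script.
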(event `Turn On/Off`
  (bind _output_get (set `self.On` (!= (`self.On`) true)))
  (if _output_get
    (for _array_element (`PrimitiveComponent.GetOverlappingActors` (`self.heat_collider`) null)
      (if (`KismetSystemLibrary.DoesImplementInterface` _array_element "/Game/Interfaces/BPI_Interaction.BPI_Interaction_C")
        (message `/Game/Interfaces/BPI_Interaction.EnterHeat` _array_element)))
    (bind (_direction _heatertrack) (`Timeline|Heater Timer` :`NewTime` 2.0 :!label _label)
      (:`Update`
        (bind _output_get_2 (set `self.Heat` _heatertrack))
        (`MaterialInstanceDynamic.SetScalarParameterValue` (`self.Material_Instance`) "EmissiveStrength" _output_get_2)))
    (else
      (for _array_element_2 (`PrimitiveComponent.GetOverlappingActors` (`self.heat_collider`) null)
        (if (`KismetSystemLibrary.DoesImplementInterface` _array_element_2 "/Game/Interfaces/BPI_Interaction.BPI_Interaction_C")
          (message `/Game/Interfaces/BPI_Interaction.ExitHeat` _array_element_2)))
      (goto _label :!via `Reverse`))))

(event `self.heat_collider.OnComponentBeginOverlap`
  (params (OverlappedComponent :type "PrimitiveComponent Object Reference") (OtherActor :type "Actor Object Reference") (OtherComp :type "PrimitiveComponent Object Reference") (OtherBodyIndex :type Integer) (bFromSweep :type Boolean) (SweepResult :type "HitResult Structure (by ref)"))
  (if (`KismetSystemLibrary.DoesImplementInterface` OtherActor "/Game/Interfaces/BPI_Interaction.BPI_Interaction_C")
    (if (`self.On`)
      (message `/Game/Interfaces/BPI_Interaction.EnterHeat` OtherActor))))

(event `self.heat_collider.OnComponentEndOverlap`
  (params (OverlappedComponent :type "PrimitiveComponent Object Reference") (OtherActor :type "Actor Object Reference") (OtherComp :type "PrimitiveComponent Object Reference") (OtherBodyIndex :type Integer))
  (if (`KismetSystemLibrary.DoesImplementInterface` OtherActor "/Game/Interfaces/BPI_Interaction.BPI_Interaction_C")
    (message `/Game/Interfaces/BPI_Interaction.ExitHeat` OtherActor)))

(fn `UserConstructionScript`
  (bind _returnvalue (`PrimitiveComponent.CreateDynamicMaterialInstance` (`self.stove_top`) 0 "/Game/Models/Stove/m_stove_top.m_stove_top" "None"))
  (set `self.Material_Instance` _returnvalue))